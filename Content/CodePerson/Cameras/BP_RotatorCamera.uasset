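; Trigger volume that rotates the CodePerson character's spring arm to a target world yaw when the character overlaps its box.
; A looping timer eases the yaw with FInterpTo, leaving pitch and roll unchanged, until the rounded value matches the target.
; On overlap it first resets an optional connected rotator, clearing that actor's timer so the two do not compete.
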(event OnComponentBeginOverlap(Box)
  (params (OverlappedComponent :type Primitive%20Component%20Object%20Reference) (OtherActor :type Actor%20Object%20Reference) (OtherComp :type Primitive%20Component%20Object%20Reference) (OtherBodyIndex :type Integer) (bFromSweep :type Boolean) (SweepResult :type Hit%20Result%20Structure%20%28by%20ref%29))
  (bind _connected (Variables|Default|GetConnected))
  (if (Class|GameplayStatics|ObjectIsA OtherActor "/Script/CodeOfPerson.CodePersonCharacter")
    (if (Utilities|IsValidSoftObjectReference _connected)
      (CallFunction|Reset (Utilities|ResolveSoftReference _connected)))
    (Variables|Default|SetSprintArm (Actor|GetComponentbyClass OtherActor "/Script/Engine.SpringArmComponent"))
    (Variables|Default|SetFinish false)
    (CallFunction|StartRotation)))

(event Custom|RotateCamera
  (bind _sprintarm (Variables|Default|GetSprintArm)
    (:then
      (if (== (Math|Float|Round (.yaw (Transformation|GetWorldRotation _sprintarm))) (Math|Float|Round (Variables|Default|GetCurrentTarget)))
        (Utilities|Time|ClearandInvalidateTimerbyHandle (Variables|Default|GetTimerHandle))
        (Variables|Default|SetFinish true)
        (Variables|Default|SetSprintArm 0)
        (else
          (Transformation|SetWorldRotation _sprintarm (Math|Rotator|MakeRotator (.roll (Transformation|GetWorldRotation (Variables|Default|GetSprintArm))) (.pitch (Transformation|GetWorldRotation (Variables|Default|GetSprintArm))) (Math|Interpolation|FInterpTo (.yaw (Transformation|GetWorldRotation (Variables|Default|GetSprintArm))) (Variables|Default|GetCurrentTarget) (Utilities|Time|GetWorldDeltaSeconds) (Variables|Default|GetInterp%20Speed))) false false))))
    (:else)))

(event Custom|StartRotation
  (bind _returnvalue (Utilities|Time|SetTimerbyEvent (EventDispatchers|CreateEvent :!event Custom|RotateCamera) (Variables|Default|GetUpdateTime) true true))
  (Variables|Default|SetTimerHandle _returnvalue))

(event EventBeginPlay
  (Variables|Default|SetCurrentTarget (Variables|Default|GetTargetZRotation)))

(fn ConstructionScript)

(fn Reset
  (Utilities|Time|ClearandInvalidateTimerbyHandle (Variables|Default|GetTimerHandle)))