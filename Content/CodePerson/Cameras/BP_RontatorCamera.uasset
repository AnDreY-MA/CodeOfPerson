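; BP_RontatorCamera is a trigger volume that turns the camera boom of a CodePersonCharacter entering its box to a target yaw.
; On overlap it caches the character's SpringArmComponent and starts a looping timer to drive the rotation.
; RotateCamera eases the arm's world yaw with FInterpTo, keeping pitch and roll, and clears the timer once yaw is within one degree below the target.
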(event OnComponentBeginOverlap(Box)
  (params (OverlappedComponent :type Primitive%20Component%20Object%20Reference) (OtherActor :type Actor%20Object%20Reference) (OtherComp :type Primitive%20Component%20Object%20Reference) (OtherBodyIndex :type Integer) (bFromSweep :type Boolean) (SweepResult :type Hit%20Result%20Structure%20%28by%20ref%29))
  (if (Class|GameplayStatics|ObjectIsA OtherActor "/Script/CodeOfPerson.CodePersonCharacter")
    (Variables|Default|SetSprintArm (Actor|GetComponentbyClass OtherActor "/Script/Engine.SpringArmComponent"))
    (bind _returnvalue (Utilities|Time|SetTimerbyEvent (EventDispatchers|CreateEvent :!event Custom|RotateCamera) (Variables|Default|GetUpdateTime) true true))
    (Variables|Default|SetTimerHandle _returnvalue)))

(event Custom|RotateCamera
  (bind _sprintarm (Variables|Default|GetSprintArm))
  (bind _targetzrotation (Variables|Default|GetTargetZRotation))
  (bind _returnvalue (Transformation|GetWorldRotation _sprintarm))
  (bind _sprintarm_2 (Variables|Default|GetSprintArm)
    (:then
      (if (Math|Float|InRange(Float) (.yaw (Transformation|GetWorldRotation _sprintarm_2)) (- _targetzrotation 1.0) _targetzrotation)
        (Utilities|Time|ClearandInvalidateTimerbyHandle (Variables|Default|GetTimerHandle))
        (else
          (Transformation|SetWorldRotation _sprintarm_2 (Math|Rotator|MakeRotator (.roll _returnvalue) (.pitch _returnvalue) (Math|Interpolation|FInterpTo (.yaw _returnvalue) (Variables|Default|GetTargetZRotation) (Utilities|Time|GetWorldDeltaSeconds) (Variables|Default|GetInterp%20Speed))) false false))))
    (:else)))

(fn ConstructionScript)