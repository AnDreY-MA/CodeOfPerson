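; BP_Box is an interactable box that slides along with the player who grabs it.
; Interact gives the player a loose Abilities.Fire tag, calls GrabBox on their BPC_Interaction and enables Tick, which starts disabled.
; Tick uses the sign of the player's world X velocity to interpolate BoxMesh along its forward vector via MoveDirection.
; Sideways movement and physics simulation are unwired, and nothing here releases the box.
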(event EventInteract
  (params (InInstigator :type Actor%20Object%20Reference))
  (Ability|GameplayEffect|AddLooseGameplayTags InInstigator (GameplayTags|MakeGameplayTagContainerfromTag "(TagName=\"Abilities.Fire\")"))
  (Default|GrabBox (Actor|GetComponentbyClass InInstigator "/Game/CodePerson/Interaction/Components/BPC_Interaction.BPC_Interaction_C"))
  (Variables|Default|SetPlayer InInstigator)
  (Actor|Tick|SetActorTickEnabled true))

(event EventTick
  (params (DeltaSeconds :type Float%20%28single-precision%29))
  (bind _player (Variables|Default|GetPlayer))
  (bind _returnvalue (Transformation|GetVelocity _player))
  (bind _returnvalue_2 (Math|Vector|Normalize _returnvalue))
  (Variables|Default|SetForward/Back (.x _returnvalue_2))
  (Variables|Default|SetRight/Left (.y _returnvalue_2))
  (Utilities|FlowControl|Sequence
    (:then_0
      (if (> (Variables|Default|GetForward/Back) 0.0)
        (Utilities|Move/Direction true (Variables|Default|GetDirection%20Speed))
        (elif (< (Variables|Default|GetForward/Back) 0.0)
          (Utilities|Move/Direction true (* (Variables|Default|GetDirection%20Speed) -1.0)))))))

(event EventBeginPlay
  (Actor|Tick|SetActorTickEnabled false))

(fn ConstructionScript)

(fn MoveDirection
  (params (Forw/Back :type Boolean) (DirectionSpeed :type Float%20%28double-precision%29))
  (Utilities|Move/Direction Forw/Back DirectionSpeed))