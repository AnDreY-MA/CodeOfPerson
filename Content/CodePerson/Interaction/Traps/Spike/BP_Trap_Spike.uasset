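; BP_Trap_Spike is a spike trap that damages actors overlapping its Box.
; Each overlap starts an async load of the damage effect class while immediately playing the spike animation and setting the Trap component's relative rotation.
; When loading completes, it applies that effect using the overlapping actor's ability system component as both source and target, then sends a hit-react gameplay event to that actor.
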(event OnComponentBeginOverlap(Box)
  (params (OverlappedComponent :type Primitive%20Component%20Object%20Reference) (OtherActor :type Actor%20Object%20Reference) (OtherComp :type Primitive%20Component%20Object%20Reference) (OtherBodyIndex :type Integer) (bFromSweep :type Boolean) (SweepResult :type Hit%20Result%20Structure%20%28by%20ref%29))
  (bind _returnvalue (Ability|GetAbilitySystemComponent OtherActor))
  (bind _trap (Variables|Default|GetTrap))
  (Utilities|AsyncLoadClassAsset (Variables|Default|GetDamage%20Effect%20Class)
    (:then
      (Components|Animation|PlayAnimation _trap "/Game/CodePerson/Interaction/Traps/Spike/AS_Spike_Down.AS_Spike_Down" false)
      (Transformation|SetRelativeRotation _trap "0.000000,0.000000,90.000000" false false))
    (:Completed
      (Class|CombatSystemFunctionLibrary|ApplyDamage (Utilities|Struct|MakeDamageEffectData (Utilities|ResolveSoftReference (Variables|Default|GetDamage%20Effect%20Class)) _returnvalue _returnvalue))
      (Ability|SendGameplayEventtoActor OtherActor "(TagName=\"Events.HitReact\")"))))

(fn ConstructionScript)