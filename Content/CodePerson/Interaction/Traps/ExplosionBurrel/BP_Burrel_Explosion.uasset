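; Explosive barrel trap that blows up when it takes any damage, firing a radial impulse and hurting a nearby Pawn.
; A sphere trace applies fire-type damage to its single hit and, if that actor has an Ability System Component, an async-loaded gameplay effect.
; The explosion Niagara system loads asynchronously alongside the trace, then spawns at the barrel, which destroys itself after a short delay.
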(event Custom|DamageShpere
  (bind _returnvalue (Transformation|GetActorLocation))
  (bind (_outhit _returnvalue_2) (Collision|SphereTraceForObjects _returnvalue _returnvalue (Variables|Default|GetRadius) (Utilities|Array|MakeArray "ObjectTypeQuery3") false 0 "None"))
  (if _returnvalue_2
    (Game|Damage|ApplyDamage (.HitActor (Collision|BreakHitResult _outhit)) 0.0 0 0 "/Game/CodePerson/Interaction/Traps/ExplosionBurrel/BP_DamageType_Fire.BP_DamageType_Fire_C")
    (Utilities|IsValid (Ability|GetAbilitySystemComponent (.HitActor (Collision|BreakHitResult _outhit)))
      (:Is%20Valid
        (Utilities|AsyncLoadClassAsset (Variables|Default|GetDamageEffect)
          (:Completed
            (GameplayEffects|ApplyGameplayEffectToSelf :self (Ability|GetAbilitySystemComponent (.HitActor (Collision|BreakHitResult _outhit))) :GameplayEffectClass (Utilities|ResolveSoftReference (Variables|Default|GetDamageEffect)))))))))

(event Game|Damage|EventAnyDamage
  (params (Damage :type Float%20%28single-precision%29) (DamageType :type Damage%20Type%20Object%20Reference) (InstigatedBy :type Controller%20Object%20Reference) (DamageCauser :type Actor%20Object%20Reference))
  (bind _returnvalue (Transformation|GetActorLocation))
  (Class|RadialForceComponent|FireImpulse (Variables|Default|GetRadialForce))
  (bind _object (Utilities|AsyncLoadAsset (Variables|Default|GetExplosion))
    (:then
      (bind (_outhit _returnvalue_2) (Collision|SphereTraceForObjects _returnvalue _returnvalue (Variables|Default|GetRadius) (Utilities|Array|MakeArray "ObjectTypeQuery3") false 0 "None"))
      (if _returnvalue_2
        (Game|Damage|ApplyDamage (.HitActor (Collision|BreakHitResult _outhit)) 0.0 0 0 "/Game/CodePerson/Interaction/Traps/ExplosionBurrel/BP_DamageType_Fire.BP_DamageType_Fire_C")
        (Utilities|IsValid (Ability|GetAbilitySystemComponent (.HitActor (Collision|BreakHitResult _outhit)))
          (:Is%20Valid
            (Utilities|AsyncLoadClassAsset (Variables|Default|GetDamageEffect)
              (:Completed
                (GameplayEffects|ApplyGameplayEffectToSelf :self (Ability|GetAbilitySystemComponent (.HitActor (Collision|BreakHitResult _outhit))) :GameplayEffectClass (Utilities|ResolveSoftReference (Variables|Default|GetDamageEffect)))))))))
    (:Completed
      (bind _asniagara_system (Utilities|Casting|CastToNiagaraSystem _object))
      (Niagara|SpawnSystematLocation _asniagara_system (Transformation|GetActorLocation) "0, 0, 0" "0.500000,0.500000,0.500000")
      (Utilities|FlowControl|Delay 0.1)
      (Actor|DestroyActor))))

(fn ConstructionScript)