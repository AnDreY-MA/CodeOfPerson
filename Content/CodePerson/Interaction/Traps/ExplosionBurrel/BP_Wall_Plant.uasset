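; BP_Wall_Plant is a plant wall obstacle that burns away when it takes fire damage.
; On damage of type BP_DamageType_Fire, it async loads a dissolve material and applies it to its cube as a dynamic material instance.
; A looping timer then advances the material's TimeValue parameter by world delta seconds until the actor destroys itself near full dissolve.
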(event Custom|Dissolve
  (bind _dynamicmaterial (Variables|Default|GetDynamicMaterial)
    (:then
      (bind _output_get (Variables|Default|SetValue (+ (Variables|Default|GetValue) (Utilities|Time|GetWorldDeltaSeconds))))
      (Rendering|Material|SetScalarParameterValue _dynamicmaterial "TimeValue" _output_get :!class /Script/Engine.MaterialInstanceDynamic)
      (if (>= (Variables|Default|GetValue) 0.95)
        (Actor|DestroyActor)))
    (:else)))

(event Game|Damage|EventAnyDamage
  (params (Damage :type Float%20%28single-precision%29) (DamageType :type Damage%20Type%20Object%20Reference) (InstigatedBy :type Controller%20Object%20Reference) (DamageCauser :type Actor%20Object%20Reference))
  (if (Class|GameplayStatics|ObjectIsA DamageType "/Game/CodePerson/Interaction/Traps/ExplosionBurrel/BP_DamageType_Fire.BP_DamageType_Fire_C")
    (Utilities|AsyncLoadAsset (Variables|Default|GetDisolveMaterial)
      (:Completed
        (bind _returnvalue (Rendering|Material|CreateDynamicMaterialInstance (Variables|Default|GetCube) 0 (Utilities|ResolveSoftReference (Variables|Default|GetDisolveMaterial)) "None" :!class /Script/Engine.PrimitiveComponent))
        (Variables|Default|SetDynamicMaterial _returnvalue)
        (Utilities|Time|SetTimerbyEvent (delegate Custom|Dissolve) 0.03 true)))))

(fn ConstructionScript)