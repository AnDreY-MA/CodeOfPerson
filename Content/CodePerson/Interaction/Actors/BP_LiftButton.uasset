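; BP_LiftButton is an interactable lift button that opens its door only when the interactor carries a key item.
; On interaction it checks the instigator's inventory for the key tag, removes one and plays the door level sequence.
; Without the key it starts the lift dialogue instead.
; An event bound to the sequence's finish appears to print a debug message.
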(event OnBeginInteracted(MamontBoxInteractable)
  (params (InInstigator :type Actor%20Object%20Reference))
  (bind _doorsequence (Variables|Default|GetDoorSequence))
  (bind _sequenceplayer (Variables|/Script/LevelSequence.LevelSequenceActor|GetSequencePlayer _doorsequence))
  (bind _returnvalue (Class|InventoryComponentInterface|GetInventoryComponent(Message) InInstigator))
  (if (Class|InventoryComponent|HasItem _returnvalue (Variables|Default|GetKeyTag))
    (Class|InventoryComponent|RemoveItem _returnvalue (Variables|Default|GetKeyTag) 1)
    (Sequencer|Player|Play _sequenceplayer :!class /Script/MovieScene.MovieSceneSequencePlayer)
    (EventDispatchers|BindEventtoOnFinished _sequenceplayer (EventDispatchers|CreateEvent :!event Custom|OnFinale))
    (else
      (CallFunction|StartNewDialogue InInstigator "/Game/CodePerson/Narrative/Dialogues/Monteaa/FromPlayer/MD_Lift.MD_Lift"))))

(event Custom|OnFinale
  (Development|PrintString "Over"))

(fn ConstructionScript)