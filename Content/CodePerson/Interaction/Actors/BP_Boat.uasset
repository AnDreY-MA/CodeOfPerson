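; BP_Boat is an interactable boat actor with front and back movement events.
; On BeginPlay it casts its TriggerBack and TriggerFront child actors to BP_Trigger_Object and binds to their OnInteract dispatchers.
; OnFront and OnBack ease the root component over a fixed time toward a GetMoveDirection target, with opposite signs.
; GetMoveDirection holds an actor-location plus signed forward-vector times SpeedStep calculation.
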(event Custom|OnFront
  (Development|PrintString "OnFront")
  (Components|MoveComponentTo (Variables|Default|GetDefaultSceneRoot) (Utilities|GetMoveDirection 1.0) "0, 0, 0" true true 1.0 false))

(event Custom|OnBack
  (Components|MoveComponentTo (Variables|Default|GetDefaultSceneRoot) (Utilities|GetMoveDirection -1.0) "0, 0, 0" true true 1.0 false))

(event EventBeginPlay
  (|CallParentFunction)
  (bind _asbp_trigger_object (Utilities|Casting|CastToBP_Trigger_Object (Variables|/Script/Engine.ChildActorComponent|GetChildActor (Variables|Default|GetTriggerBack))))
  (EventDispatchers|BindEventtoOnInteract _asbp_trigger_object (EventDispatchers|CreateEvent :!event Custom|OnBack))
  (bind _asbp_trigger_object_2 (Utilities|Casting|CastToBP_Trigger_Object (Variables|/Script/Engine.ChildActorComponent|GetChildActor (Variables|Default|GetTriggerFront))))
  (EventDispatchers|BindEventtoOnInteract _asbp_trigger_object_2 (EventDispatchers|CreateEvent :!event Custom|OnFront)))

(fn ConstructionScript)