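; BP_Pushable is an interactable actor that snaps an instigator to a predefined push spot and starts a push through its BP_Push_Component.
; Construction draws an arrow for each PushTransform entry.
; On interaction, Handle picks the closest spot within the component's push range.
; A capsule trace checks overlap and walkable floor, and a line trace checks obstructions before the instigator is moved and BeginPushBP is called.
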(event OnBeginInteracted(MamontBoxInteractable)
  (params (InInstigator :type Actor%20Object%20Reference))
  (CallFunction|Handle InInstigator))

(event OnEndInteracted(MamontBoxInteractable)
  (params (InInstigator :type Actor%20Object%20Reference)))

(fn ConstructionScript
  (for _array_element (Variables|Default|GetPushTransform)
    (AddComponent|AddArrowComponent false _array_element)))

(fn Handle
  (params (InInstigator :type Actor%20Object%20Reference))
  (bind _returnvalue (Actor|GetComponentbyClass InInstigator "/Game/CodePerson/Interaction/Actors/Pushable/BP_Push_Component.BP_Push_Component_C"))
  (bind _returnvalue_2 (Actor|GetComponentbyClass InInstigator "/Script/Engine.CapsuleComponent"))
  (Utilities|IsValid _returnvalue
    (:Is%20Valid
      (bind _output_get (LocalVariables|SetPushComponent _returnvalue))
      (bind _returnvalue_3 (CallFunction|FindClosestPushTransformIndex (Math|Conversions|ToVector2D(Vector) (Transformation|GetActorLocation InInstigator)) (Default|GetPushRange _output_get)))
      (if (>= _returnvalue_3 0)
        (Development|PrintString (Utilities|String|Append "Index" (Utilities|String|ToString(Integer) _returnvalue_3)))
        (LocalVariables|SetInstigatorNewTransform (|CalculateNewTransform _returnvalue_3))
        (bind _outhit (Collision|CapsuleTraceByChannel (+ (.location (LocalVariables|GetInstigatorNewTransform)) "0.000000,0.000000,70.000000") (- (.location (LocalVariables|GetInstigatorNewTransform)) "0.000000,0.000000,100.000000") (Components|Capsule|GetScaledCapsuleRadius _returnvalue_2) (Components|Capsule|GetScaledCapsuleHalfHeight _returnvalue_2) "TraceTypeQuery1" false (Utilities|Array|MakeArray InInstigator) "ForDuration"))
        (if (not (.bInitialOverlap (Collision|BreakHitResult _outhit)))
          (if (< (Class|CharacterMovementComponent|GetWalkableFloorZ (Actor|GetComponentbyClass InInstigator "/Script/Engine.CharacterMovementComponent")) (.Z (Math|Vector|BreakVector (.ImpactNormal (Collision|BreakHitResult _outhit)))))
            (bind _returnvalue_4 (Collision|LineTraceByChannel (Transformation|GetActorLocation) (.location (LocalVariables|GetInstigatorNewTransform)) "TraceTypeQuery1" false (Utilities|Array|MakeArray InInstigator) "None"))
            (if (not _returnvalue_4)
              (Transformation|SetActorTransform InInstigator (Math|Transform|MakeTransform (.location (LocalVariables|GetInstigatorNewTransform)) (.rotation (LocalVariables|GetInstigatorNewTransform)) (.scale (LocalVariables|GetInstigatorNewTransform))))
              (Default|BeginPushBP (LocalVariables|GetPushComponent) self))))))))

(fn FindTransform
  (params (InInstigatorLocation :type Vector%202D%20Structure) (InPushRange :type Float%20%28double-precision%29))
  (for (_array_element _array_index) (Variables|Default|GetPushTransform)
    (LocalVariables|SetCurrentTransformIndex _array_index)
    (bind _output_get (LocalVariables|SetCurrentDistance (Class|KismetMathLibrary|DistanceSquared2D (Math|Conversions|ToVector2D(Vector) (Math|Transform|TransformLocation (Transformation|GetActorTransform) (.Location (Math|Transform|BreakTransform _array_element)))) InInstigatorLocation)))
    (if (< _output_get (Math|Float|Square InPushRange))
      (if (or (< (LocalVariables|GetCurrentDistance) (LocalVariables|GetClosestDistance)) (< (LocalVariables|GetClosestTransformIndex) 0))
        (LocalVariables|SetClosestTransformIndex (LocalVariables|GetCurrentTransformIndex))
        (LocalVariables|SetClosestDistance (LocalVariables|GetCurrentDistance)))))
  (return (LocalVariables|GetClosestTransformIndex)))

(fn FindClosestPushTransformIndex
  (params (InInstigatorLocation :type Vector%202D%20Structure%20%28by%20ref%29) (InPushRange :type Float%20%28single-precision%29))
  (bind _outbestindex (CallFunction|FindTransform InInstigatorLocation InPushRange))
  (return _outbestindex))