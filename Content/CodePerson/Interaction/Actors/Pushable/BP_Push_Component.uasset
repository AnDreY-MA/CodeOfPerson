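; Character component that lets its owner grab and push an object around.
; BeginPushBP attaches the character to the object and enables ticking; EndPushBP detaches it and disables ticking, with both updating a hold gameplay tag.
; Tick remaps stored forward/right input by rounded character yaw range, then moves the object with a swept world offset, carrying the attached character along.
; A separate moving tag follows whether that input is non-zero.
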(event EventTick
  (params (DeltaSeconds :type Float%20%28single-precision%29))
  (bind _character (Variables|Default|GetCharacter))
  (bind _movingtag (Variables|Settings|GetMovingTag))
  (CallFunction|Pushing DeltaSeconds)
  (if (Variables|Default|GetIsMovingAnObject)
    (Ability|GameplayEffect|AddLooseGameplayTags _character _movingtag)
    (else
      (Ability|GameplayEffect|RemoveLooseGameplayTags _character _movingtag))))

(event EventBeginPlay
  (bind _ascharacter (Utilities|Casting|CastToCharacter (Components|GetOwner)))
  (Variables|Default|SetCharacter _ascharacter)
  (Development|PrintString (Utilities|String|ToString(Boolean) (Variables|Default|GetIsMovingAnObject))))

(fn GetPushRange
  (return (Variables|Settings|GetPushRange)))

(fn BeginPushBP
  (params (InPushObejct :type BP%20Pushable%20Object%20Reference))
  (Variables|Default|GetPushableObject
    (:then)
    (:else
      (bind _output_get (Variables|Default|SetPushableObject InPushObejct))
      (Transformation|AttachActorToActor (Variables|Default|GetCharacter) _output_get "None" "KeepWorld" "KeepWorld" "KeepWorld" true)
      (Variables|/Script/Engine.CharacterMovementComponent|SetbOrientRotationToMovement (Variables|/Script/Engine.Character|GetCharacterMovement (Variables|Default|GetCharacter)) true)
      (Components|Tick|SetComponentTickEnabled true)
      (Ability|GameplayEffect|AddLooseGameplayTags (Variables|Default|GetCharacter) (Variables|Settings|GetHoldObjectTag)))))

(fn IsHoldingObject
  (return (Utilities|IsValid (Variables|Default|GetPushableObject))))

(fn SetDirectionValues
  (params (InForward :type Float%20%28double-precision%29) (InRight :type Float%20%28double-precision%29))
  (Variables|Default|SetForwardMove InForward)
  (Variables|Default|SetRightMove InRight))

(fn GetDeltaLocation
  (params (InDeltaSecond :type Float%20%28double-precision%29) (InForward :type Float%20%28double-precision%29) (InRight :type Float%20%28double-precision%29))
  (Variables|Default|SetIsMovingAnObject (or (!= InForward 0.0) (!= InRight 0.0)))
  (return (+ (* (* (Transformation|GetActorForwardVector (Variables|Default|GetCharacter)) InForward) (* InDeltaSecond (Variables|Settings|GetPushSpeed))) (* (* InDeltaSecond (Variables|Settings|GetPushSpeed)) (* (Transformation|GetActorRightVector (Variables|Default|GetCharacter)) InRight)))))

(fn Pushing
  (params (InDelta :type Float%20%28double-precision%29))
  (bind _output_get (Variables|Default|SetCurrentActorZRotation (Math|Conversions|ToFloat(Integer) (Math|Float|Round (.yaw (Transformation|GetActorRotation (Variables|Default|GetCharacter)))))))
  ;[1 1 1] Up
  (Development|PrintString (Utilities|String|ToString(Float) _output_get))
  (if (and (>= _output_get 0.0) (< _output_get 9e+01))
    (Development|PrintString "UP")
    (Utilities|AddOffset InDelta (Variables|Default|GetForwardMove) (Variables|Default|GetRightMove))
    (else
      ;[1 1 1] Right
      (if (and (>= (Variables|Default|GetCurrentActorZRotation) 8e+01) (< (Variables|Default|GetCurrentActorZRotation) 1.7e+02))
        (Utilities|AddOffset InDelta (Variables|Default|GetRightMove) (* (Variables|Default|GetForwardMove) -1.0))
        (else
          ;[1 1 1] Left
          (if (and (>= (Variables|Default|GetCurrentActorZRotation) -9e+01) (< (Variables|Default|GetCurrentActorZRotation) 0.0))
            (Utilities|AddOffset InDelta (* (Variables|Default|GetRightMove) -1.0) (Variables|Default|GetForwardMove))
            (else
              ;[1 1 1] Down
              (if (>= (Variables|Default|GetCurrentActorZRotation) 1.8e+02)
                (Development|PrintString "Down")
                (Utilities|AddOffset InDelta (* (Variables|Default|GetForwardMove) -1.0) (* (Variables|Default|GetRightMove) -1.0))))))))))

(fn EndPushBP
  (Utilities|IsValid (Variables|Default|GetPushableObject)
    (:Is%20Valid
      (Variables|Default|SetPushableObject 0)
      (Variables|Default|SetIsMovingAnObject false)
      (Transformation|DetachFromActor (Variables|Default|GetCharacter) "KeepWorld" "KeepWorld" "KeepWorld")
      (Variables|/Script/Engine.CharacterMovementComponent|SetbOrientRotationToMovement (Variables|/Script/Engine.Character|GetCharacterMovement (Variables|Default|GetCharacter)) true)
      (Components|Tick|SetComponentTickEnabled false)
      (Ability|GameplayEffect|RemoveLooseGameplayTags (Variables|Default|GetCharacter) (Variables|Settings|GetHoldObjectTag)))))