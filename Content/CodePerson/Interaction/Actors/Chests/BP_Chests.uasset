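; BP_Chests is an interactable loot chest that gives the player a count of an item and saves its opened state.
; Interaction activates the instigator's OpenChest ability by tag; on BeginPlay, an already-opened chest strips its interaction and effect components.
; Open removes interaction components, async-loads a Niagara loot effect, and adds the item to inventory.
; Tick runs only briefly, feeding the player's location to the effect before it is destroyed.
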(event OnBeginInteracted(MamontBoxInteractable)
  (params (InInstigator :type Actor%20Object%20Reference))
  (Abilities|TryActivateAbilitiesbyTag (Ability|GetAbilitySystemComponent InInstigator) (GameplayTags|MakeGameplayTagContainerfromTag "(TagName=\"Abilities.General.OpenChest\")") true))

(event EventOpen
  (bind _ns_lootdrop (Variables|Default|GetNS_LootDrop))
  (Audio|SpawnSound2D (Variables|Default|GetOpenSound) 1.0 1.0 0.0 0)
  (Variables|Default|SetData (Utilities|Struct|MakeS_Chests true))
  (Components|DestroyComponent (Variables|Default|GetPlane))
  (bind _object (Utilities|AsyncLoadAsset (Variables|Default|GetLootEffect))
    (:Completed
      (bind _asniagara_system (Utilities|Casting|CastToNiagaraSystem _object))
      (Class|NiagaraComponent|SetAsset _ns_lootdrop _asniagara_system true)
      (Class|NiagaraComponent|SetVariableInt _ns_lootdrop "Count" (Variables|Default|GetCountLoot))
      (Components|Activation|SetActive (Variables|Default|GetNS_LootDrop) true true)
      (Utilities|FlowControl|Delay 0.2)
      (Utilities|FlowControl|Sequence
        (:then_0
          (Actor|Tick|SetActorTickEnabled true)
          (Utilities|FlowControl|Delay 2.0)
          (Actor|Tick|SetActorTickEnabled false)
          (Components|DestroyComponent (Variables|Default|GetNS_LootDrop)))
        (:then_1
          (Audio|SpawnSound2D (Variables|Default|GetCoinsSound) 1.0 1.0 0.0 0)
          (bind _returnvalue (Class|InventoryComponentInterface|GetInventoryComponent(Message) (Game|GetPlayerCharacter 0)))
          (Class|InventoryComponent|AddItem _returnvalue (Variables|Default|GetItem) (Variables|Default|GetCountLoot)))))))

(event EventTick
  (params (DeltaSeconds :type Float%20%28single-precision%29))
  (Niagara|SetNiagaraVariable(Vector3) (Variables|Default|GetNS_LootDrop) "ActorLocation" (Transformation|GetActorLocation (Game|GetPlayerCharacter 0))))

(event EventBeginPlay
  (|CallParentFunction)
  (bind _outdata (Utilities|LoadDataforObject self)
    (:true
      (bind _value (Class|StructUtilsFunctionLibrary|GetInstancedStructValue _outdata)
        (:Valid
          (if (Utilities|Struct|BreakS_Chests _value)
            (Components|DestroyComponent (Variables|Default|GetPlane))))))))

(fn ConstructionScript)

(fn GetSave
  (bind _returnvalue (Class|StructUtilsFunctionLibrary|MakeInstancedStruct (Variables|Default|GetData)))
  (return (Utilities|Struct|MakeS_SaveActorsData (Utilities|String|StringToName (Utilities|GetObjectName self)) _returnvalue)))

(fn GetSaveDataPlayer
  (return ""))

(fn IsShouldSave
  (return true))