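; BP_ButtonFloor is a floor button that plays sequences while an actor overlaps its TopButton component.
; The first overlapping actor is stored, the button's ActorSequence and the linked Depenced sequence play forward, and the top turns red.
; When that stored actor leaves, both sequences reverse, the top turns green, and the reference clears, so other overlaps are ignored while one actor holds it.
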(event OnComponentBeginOverlap(TopButton)
  (params (OverlappedComponent :type Primitive%20Component%20Object%20Reference) (OtherActor :type Actor%20Object%20Reference) (OtherComp :type Primitive%20Component%20Object%20Reference) (OtherBodyIndex :type Integer) (bFromSweep :type Boolean) (SweepResult :type Hit%20Result%20Structure%20%28by%20ref%29))
  (Variables|Default|GetOther%20Actor
    (:then)
    (:else
      (Variables|Default|SetOther%20Actor OtherActor)
      (Sequencer|Player|Play (Variables|/Script/ActorSequence.ActorSequenceComponent|GetSequencePlayer (Variables|Default|GetActorSequence)) :!class /Script/MovieScene.MovieSceneSequencePlayer)
      (Rendering|Material|SetMaterial (Variables|Default|GetTopButton) 0 "/Game/CodePerson/Materials/Levels/MI_Color_Red.MI_Color_Red")
      (Sequencer|Player|Play (Variables|/Script/LevelSequence.LevelSequenceActor|GetSequencePlayer (Variables|Default|GetDepenced)) :!class /Script/MovieScene.MovieSceneSequencePlayer))))

(event OnComponentEndOverlap(TopButton)
  (params (OverlappedComponent :type Primitive%20Component%20Object%20Reference) (OtherActor :type Actor%20Object%20Reference) (OtherComp :type Primitive%20Component%20Object%20Reference) (OtherBodyIndex :type Integer))
  (Variables|Default|GetOther%20Actor
    (:then
      (if (== OtherActor (Variables|Default|GetOther%20Actor))
        (Class|MovieSceneSequencePlayer|PlayReverse (Variables|/Script/ActorSequence.ActorSequenceComponent|GetSequencePlayer (Variables|Default|GetActorSequence)))
        (Rendering|Material|SetMaterial (Variables|Default|GetTopButton) 0 "/Game/CodePerson/Materials/Levels/MI_Color_Green.MI_Color_Green")
        (Variables|Default|SetOther%20Actor 0)
        (Class|MovieSceneSequencePlayer|PlayReverse (Variables|/Script/LevelSequence.LevelSequenceActor|GetSequencePlayer (Variables|Default|GetDepenced)))))
    (:else)))

(fn ConstructionScript)