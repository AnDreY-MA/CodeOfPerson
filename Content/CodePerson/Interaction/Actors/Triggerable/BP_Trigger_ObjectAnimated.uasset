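; Triggerable interaction actor that plays an animation on a referenced world object when interacted with.
; On interact, it checks the soft reference to the target object, async loads it, then plays that object's SequencePlayer.
; A delayed self-trigger of the interaction is left disconnected and never runs.
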(event Custom|OnInteract
  (if (Utilities|IsValidSoftObjectReference (Variables|Default|GetAnimateObject))
    (Utilities|AsyncLoadAsset (Variables|Default|GetAnimateObject)
      (:Completed
        (Sequencer|Player|Play (Variables|/Script/LevelSequence.LevelSequenceActor|GetSequencePlayer (Utilities|ResolveSoftReference (Variables|Default|GetAnimateObject))) :!class /Script/MovieScene.MovieSceneSequencePlayer)))))

(event Game|Damage|EventAnyDamage
  (params (Damage :type Float%20%28single-precision%29) (DamageType :type Damage%20Type%20Object%20Reference) (InstigatedBy :type Controller%20Object%20Reference) (DamageCauser :type Actor%20Object%20Reference)))

(event EventBeginPlay)

(fn ConstructionScript)