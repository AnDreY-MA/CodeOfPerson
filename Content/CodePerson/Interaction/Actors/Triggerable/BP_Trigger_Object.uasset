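; BP_Trigger_Object is an interaction trigger that fires when damaged, interacted with or activated through an editor event.
; Each activation calls OnInteract, then forwards Interact to its Dependers reference if valid.
; If AnimateObject is set, it async-loads that soft reference and toggles its SequencePlayer between forward and reverse playback using the First flag.
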(event Custom|Interact
  (bind _animateobject (Variables|Default|GetAnimateObject))
  (bind _output (Utilities|ResolveSoftReference _animateobject))
  (bind _sequenceplayer (Variables|/Script/LevelSequence.LevelSequenceActor|GetSequencePlayer _output))
  (Default|CallOnInteract)
  (bind _dependers (Variables|Default|GetDependers)
    (:then
      (CallFunction|Interact _dependers))
    (:else
      _))
  (if (Utilities|IsValidSoftObjectReference (Variables|Default|GetAnimateObject))
    (Utilities|AsyncLoadAsset (Variables|Default|GetAnimateObject)
      (:Completed
        (if (Variables|Default|GetFirst)
          (Sequencer|Player|Play _sequenceplayer :!class /Script/MovieScene.MovieSceneSequencePlayer)
          (Variables|Default|SetFirst false)
          (else
            (Class|MovieSceneSequencePlayer|PlayReverse _sequenceplayer)
            (Variables|Default|SetFirst true)))))))

(event Custom|ActivateInEditor
  (CallFunction|Interact))

(event Game|Damage|EventAnyDamage
  (params (Damage :type Float%20%28single-precision%29) (DamageType :type Damage%20Type%20Object%20Reference) (InstigatedBy :type Controller%20Object%20Reference) (DamageCauser :type Actor%20Object%20Reference))
  (CallFunction|Interact))

(event EventBeginPlay)

(fn ConstructionScript)