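; Base or standalone pickup item actor that goes into the instigator's inventory and persists its collected state through saves.
; Interaction adds one item by tag to the InventoryComponent, destroys the widget, interactable and mesh components, and flags it as taken.
; The actor itself remains so GetSave can store that flag in an instanced struct keyed by object name.
; On BeginPlay it loads this data and destroys itself if already collected.
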(event OnBeginInteracted(MamontBoxInteractable)
  (params (InInstigator :type Actor%20Object%20Reference))
  (CallFunction|InteractItem InInstigator))

(event Custom|InteractItem
  (params (InInstigator :type Actor%20Object%20Reference))
  (bind _returnvalue (Actor|GetComponentbyClass InInstigator "/Script/CodeOfPerson.InventoryComponent"))
  (Utilities|IsValid _returnvalue
    (:Is%20Valid
      (Class|InventoryComponent|AddItem _returnvalue (Variables|Default|GetItemName) 1)
      (Components|DestroyComponent (Variables|Default|GetWidgetComponent))
      (Variables|Default|SetItemInstanced (Utilities|Struct|MakeS_ItemInstanced true)))))

(event EventBeginPlay
  (|CallParentFunction)
  (bind _outdata (Utilities|LoadDataforObject self)
    (:true
      (bind _value (Class|StructUtilsFunctionLibrary|GetInstancedStructValue _outdata)
        (:Valid
          (if (Utilities|Struct|BreakS_ItemInstanced _value)
            (Development|PrintString "Hello" true true "(R=1.000000,G=0.265167,B=0.000000,A=1.000000)" 1e+01)
            (Actor|DestroyActor)))))))

(fn ConstructionScript)

(fn GetSave
  (Development|PrintString "Get Item")
  (bind _returnvalue (Class|StructUtilsFunctionLibrary|MakeInstancedStruct (Variables|Default|GetItemInstanced)))
  (return (Utilities|Struct|MakeS_SaveActorsData (Utilities|String|StringToName (Utilities|GetObjectName self)) _returnvalue)))

(fn GetSaveDataPlayer
  (return ""))

(fn IsShouldSave
  (return true))