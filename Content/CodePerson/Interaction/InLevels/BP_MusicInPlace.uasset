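; BP_MusicInPlace is a trigger volume that plays location-based music while the player character is inside its box.
; On begin overlap by a CodePersonCharacter, it calls PlayMusic on the GameMode's AC_SoundComponent, passing its Key, FadeOut and FadeIn variables.
; On end overlap, it calls Stop on that same component, so playback is handled centrally rather than by the volume.
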(event OnComponentBeginOverlap(Box)
  (params (OverlappedComponent :type Primitive%20Component%20Object%20Reference) (OtherActor :type Actor%20Object%20Reference) (OtherComp :type Primitive%20Component%20Object%20Reference) (OtherBodyIndex :type Integer) (bFromSweep :type Boolean) (SweepResult :type Hit%20Result%20Structure%20%28by%20ref%29))
  (if (Class|GameplayStatics|ObjectIsA OtherActor "/Script/CodeOfPerson.CodePersonCharacter")
    (Default|PlayMusic (Actor|GetComponentbyClass (Game|GetGameMode) "/Game/CodePerson/GameModes/AC_SoundComponent.AC_SoundComponent_C") (Variables|Default|GetKey) (Variables|Default|GetFade%20Out) (Variables|Default|GetFade%20In))))

(event OnComponentEndOverlap(Box)
  (params (OverlappedComponent :type Primitive%20Component%20Object%20Reference) (OtherActor :type Actor%20Object%20Reference) (OtherComp :type Primitive%20Component%20Object%20Reference) (OtherBodyIndex :type Integer))
  (if (Class|GameplayStatics|ObjectIsA OtherActor "/Script/CodeOfPerson.CodePersonCharacter")
    (Default|Stop (Actor|GetComponentbyClass (Game|GetGameMode) "/Game/CodePerson/GameModes/AC_SoundComponent.AC_SoundComponent_C"))))

(fn ConstructionScript)