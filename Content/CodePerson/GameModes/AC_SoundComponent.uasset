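; Actor component that manages background music, filed with the game modes.
; On BeginPlay it spawns BeginSound as a persistent 2D sound, reused by PlayMusic to fade out, swap to a track looked up by key in Musics, and fade in.
; Stop and Resume call fades followed immediately by Stop or Play, and EndPlay destroys the sound.
; Without a BeginSound no audio component is created for later calls.
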(event Custom|PlayMusic
  (params (Key :type Gameplay%20Tag%20Structure%20%28by%20ref%29) (FadeOut :type Float%20%28single-precision%29) (FadeIn :type Float%20%28single-precision%29))
  (bind _musics (Variables|Default|GetMusics))
  (bind _currentsound (Variables|Default|GetCurrentSound))
  (bind (_value _returnvalue) (Utilities|Map|Find _musics Key))
  (if _returnvalue
    (bind _currentsound_2 (Variables|Default|GetCurrentSound)
      (:then
        (Audio|Components|Audio|FadeOut _currentsound_2 FadeOut 0.0 "Linear" :!class /Script/Engine.AudioComponent))
      (:else
        _))
    (Utilities|FlowControl|Delay FadeOut)
    (Audio|Components|Audio|SetSound _currentsound _value)
    (Audio|Components|Audio|FadeIn _currentsound FadeIn 1.0 0.0 "Linear" :!class /Script/Engine.AudioComponent)))

(event Custom|Stop
  (bind _currentsound (Variables|Default|GetCurrentSound))
  (Audio|Components|Audio|FadeOut _currentsound 5.0 0.0 "Linear" :!class /Script/Engine.AudioComponent)
  (Audio|Components|Audio|Stop _currentsound))

(event Custom|Resume
  (bind _currentsound (Variables|Default|GetCurrentSound))
  (Audio|Components|Audio|FadeIn _currentsound 3.0 1.0 0.0 "Linear" :!class /Script/Engine.AudioComponent)
  (Audio|Components|Audio|Play _currentsound 0.0))

(event EventBeginPlay
  (bind _beginsound (Variables|Default|GetBeginSound)
    (:then
      (bind _returnvalue (Audio|SpawnSound2D _beginsound 1.0 1.0 0.0 0 false false))
      (Variables|Default|SetCurrentSound _returnvalue))
    (:else)))

(event EventEndPlay
  (params (EndPlayReason :type EEndPlayReason%20Enum :default "Destroyed"))
  (|CallParentFunction EndPlayReason)
  (bind _currentsound (Variables|Default|GetCurrentSound)
    (:then
      (Components|DestroyComponent _currentsound))
    (:else)))