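; BP_FixerBridge is an actor that drives a Manager's current time from the player's proximity, apparently to repair a destructed bridge.
; On BeginPlay it caches the CodePersonCharacter, then each Tick scales its distance to that player by a multiplier and passes the result to the Manager as the current time.
; Once that value falls to FinalResult or below, the actor destroys itself.
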(event EventBeginPlay
  (bind _returnvalue (Actor|GetActorOfClass "/Script/CodeOfPerson.CodePersonCharacter"))
  (Variables|Default|SetPlayer _returnvalue))

(event EventTick
  (params (DeltaSeconds :type Float%20%28single-precision%29))
  (Variables|Default|SetCurrentTime (* (Transformation|GetDistanceTo (Variables|Default|GetPlayer)) (Variables|Default|GetMultiplyer)))
  (Class|ChaosCacheManager|SetCurrentTime (Variables|Default|GetManager) (Variables|Default|GetCurrentTime))
  (if (<= (Variables|Default|GetCurrentTime) (Variables|Default|GetFinalResult))
    (Actor|DestroyActor)))

(fn ConstructionScript)