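; AI controller for the Bunny boss enemy, extending a parent enemy controller.
; On begin play it deactivates its perception stimuli source.
; SetTargetPlayer makes the first player the target, notifies the combat state component, and gives the controlled pawn a one-shot gameplay ability that, by its name, adds a status bar.
; It also exposes its CombatUI component through a getter.
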(event Custom|SetTargetPlayer
  (bind _returnvalue (Game|GetPlayerCharacter 0))
  (Class|CombatEnemyController|UpdateTargetActor _returnvalue)
  (Class|CombatEnemyStateComponent|DetectTarget (Variables|Default|GetCombatStateComponent) _returnvalue)
  (Class|AbilitySystemComponent|GiveAbilityandActivateOnce (Ability|GetAbilitySystemComponent (Pawn|GetControlledPawn)) "/Game/CodePerson/AbilitiySystem/Abilities/GA_AddStatusBar.GA_AddStatusBar_C" 0 -1))

(event EventBeginPlay
  (|CallParentFunction)
  (Components|Activation|Deactivate (Variables|Default|GetPerceptionStimuliSource)))

(fn ConstructionScript
  (|CallParentFunction))

(fn GetCombatUIComponent
  (return (Variables|Default|GetCombatUI)))