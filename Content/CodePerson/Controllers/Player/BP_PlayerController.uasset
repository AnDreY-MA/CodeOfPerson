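; Player controller that adds a blood screen widget behind other viewport UI and handles dialogue and pause input.
; It tracks dialogue state through start and close events from the Mountea Dialogue Manager on the PlayerState.
; The interaction input skips the current row during dialogue, while pause freezes the game and opens the HUD menu.
; It also exposes its PersonComponent; attack input only prints a debug string.
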(event Custom|OnDialogueStart
  (params (Context :type Mountea%20Dialogue%20Context%20Object%20Reference))
  (Variables|Default|SetIsDialogue true)
  (Development|PrintString (Utilities|String|Append "IsDialogue: " (Utilities|String|ToString(Boolean) (Variables|Default|GetIsDialogue)))))

(event Custom|OnDialogueFinish
  (params (Context :type Mountea%20Dialogue%20Context%20Object%20Reference))
  (Variables|Default|SetIsDialogue false)
  (Development|PrintString (Utilities|String|Append "IsDialogue: " (Utilities|String|ToString(Boolean) (Variables|Default|GetIsDialogue)))))

(event Input|EnhancedActionEvents|EnhancedInputActionIA_Interaction
  (params (ActionValue :type Boolean) (ElapsedSeconds :type Float%20%28double-precision%29) (TriggeredSeconds :type Float%20%28double-precision%29) (InputAction :type Input%20Action%20Object%20Reference :default "/Game/CodePerson/Controllers/Player/Input/Actions/IA_Interaction.IA_Interaction"))
  (:Started
    (if (Variables|Default|GetIsDialogue)
      (Class|MounteaDialogueManagerInterface|SkipDialogueRow (Actor|GetComponentbyClass (Variables|Default|GetPlayerState) "/Script/MounteaDialogueSystem.MounteaDialogueManager")))))

(event Input|EnhancedActionEvents|EnhancedInputActionIA_Pause
  (params (ActionValue :type Boolean) (ElapsedSeconds :type Float%20%28double-precision%29) (TriggeredSeconds :type Float%20%28double-precision%29) (InputAction :type Input%20Action%20Object%20Reference :default "/Game/CodePerson/Controllers/Player/Input/Actions/IA_Pause.IA_Pause"))
  (Game|SetGamePaused true)
  (Class|MamontHUDInterface|OpenMenu(Message) (HUD|GetHUD)))

(event Input|EnhancedActionEvents|EnhancedInputActionIA_Attack
  (params (ActionValue :type Boolean) (ElapsedSeconds :type Float%20%28double-precision%29) (TriggeredSeconds :type Float%20%28double-precision%29) (InputAction :type Input%20Action%20Object%20Reference :default "/Game/CodePerson/Controllers/Player/Input/Actions/IA_Attack.IA_Attack"))
  (Development|PrintString "Hello"))

(event EventBeginPlay
  (bind _playerstate (Variables|Default|GetPlayerState))
  (bind _returnvalue (Actor|GetComponentbyClass _playerstate "/Script/MounteaDialogueSystem.MounteaDialogueManager"))
  (|CallParentFunction)
  (EventDispatchers|BindEventtoOnDialogueStarted _returnvalue (EventDispatchers|CreateEvent :!event Custom|OnDialogueStart))
  (EventDispatchers|BindEventtoOnDialogueClosed _returnvalue (EventDispatchers|CreateEvent :!event Custom|OnDialogueFinish))
  (bind _returnvalue_2 (UserInterface|CreateWidget "/Game/CodePerson/UMG/WBP_BloodScreen.WBP_BloodScreen_C" self))
  (UserInterface|Viewport|AddtoViewport _returnvalue_2 -10))

(fn ConstructionScript)

(fn GetPersonComponent
  (return (Variables|Default|GetPersonComponent)))