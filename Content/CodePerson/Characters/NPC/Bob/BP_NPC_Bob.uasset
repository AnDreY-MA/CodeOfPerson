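; BP_NPC_Bob is an NPC Blueprint whose interaction box is tied to the destruction of a referenced Enemy actor.
; On BeginPlay it binds to the Enemy's OnDestroyed event and deactivates every component on its controller.
; When the Enemy is destroyed, MamontBoxInteractable switches to query-only collision.
; Overlaps with that box only print the other actor's name, as a debug placeholder.
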(event OnComponentBeginOverlap(MamontBoxInteractable)
  (params (OverlappedComponent :type Primitive%20Component%20Object%20Reference) (OtherActor :type Actor%20Object%20Reference) (OtherComp :type Primitive%20Component%20Object%20Reference) (OtherBodyIndex :type Integer) (bFromSweep :type Boolean) (SweepResult :type Hit%20Result%20Structure%20%28by%20ref%29))
  (Development|PrintString (Utilities|GetDisplayName OtherActor)))

(event Custom|OnDestroyed_Event
  (params (DestroyedActor :type Actor%20Object%20Reference))
  (Collision|SetCollisionEnabled (Variables|Default|GetMamontBoxInteractable) "QueryOnly")
  (Development|PrintString "Hello"))

(event EventBeginPlay
  (|CallParentFunction)
  (Game|AssignOnDestroyed (Variables|Default|GetEnemy) (delegate Custom|OnDestroyed_Event))
  (for _array_element (Actor|GetComponentsByClass (Pawn|GetController) "/Script/Engine.ActorComponent")
    (Components|Activation|SetActive _array_element false false)))

(fn ConstructionScript
  (|CallParentFunction))