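; BP_Sheep is a quest NPC that collects apples from the player.
; After the first dialogue, interaction only proceeds when the player's key item is an apple, which it removes and counts.
; Each delivery short of the maximum async-loads and spawns another apple at a random, non-repeating AppleItems location.
; The final one completes the quest, destroying one door, revealing another with collision and triggering its spawners.
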(event OnBeginInteracted(MamontBoxInteractable)
  (params (InInstigator :type Actor%20Object%20Reference))
  (bind _returnvalue (Actor|GetComponentbyClass InInstigator "/Script/CodeOfPerson.InventoryComponent"))
  (if (Variables|Default|GetIsFirstDialogue)
    (Variables|Default|SetIsFirstDialogue false)
    (|CallParentFunction InInstigator :!label _label)
    (if (== (Variables|Default|GetAppleCount) (Variables|Default|GetMaxAppleTaken))
      (CallFunction|FinishQuest)
      (elif (!= (Variables|Default|GetAppleCount) 0)
        (CallFunction|SpawnRandomApple)))
    (elif (== (Class|InventoryComponent|GetKeyItem _returnvalue) (GameplayTags|MakeLiteralGameplayTag "(TagName=\"Items.Apple\")"))
      (Math|Integer|IncrementInt (Variables|Default|GetAppleCount)
        (:%20%20
          (Class|InventoryComponent|RemoveItem _returnvalue (GameplayTags|MakeLiteralGameplayTag "(TagName=\"Items.Apple\")"))
          (goto _label))))))

(event Custom|SpawnRandomApple
  (bind _appleitems (Variables|Default|GetAppleItems))
  (bind (_outitem _outindex) (Utilities|Array|Random _appleitems))
  (bind _class (Utilities|AsyncLoadClassAsset (Variables|Default|GetAppleClass))
    (:Completed
      (bind _asactor (Utilities|Casting|CastToActorClass _class))
      (Game|SpawnActorfromClass _asactor (Math|Transform|MakeTransform (Transformation|GetActorLocation _outitem) "0, 0, 0" "1.000000,1.000000,1.000000") "Undefined" "MultiplyWithRoot" 0 0)
      (Utilities|Array|RemoveIndex (Variables|Default|GetAppleItems) _outindex))))

(fn ConstructionScript)

(fn StartDialogue
  (|CallParentFunction))

(fn FinishQuest
  (bind _closedoor (Variables|Default|GetCloseDoor))
  (Actor|DestroyActor (Variables|Default|GetDestroyDoor))
  (Collision|SetCollisionEnabled (Actor|GetComponentbyClass _closedoor "/Script/Engine.PrimitiveComponent") "QueryAndPhysics")
  (Rendering|SetActorHiddenInGame _closedoor false)
  (for _array_element (Variables|Default|GetSpawner)
    (Class|Spawner|Spawn _array_element)))