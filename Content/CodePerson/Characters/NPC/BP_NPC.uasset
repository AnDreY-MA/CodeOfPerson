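; BP_NPC is an NPC that the player can talk to through a box interactable and a dialogue speaker component.
; On BeginPlay it binds to the game state's combat manager event for all enemy characters dying.
; OnMayTalk enables query-only collision on the interactable.
; Interacting starts the NPC's owned dialogue with the instigator's speaker component and prints a debug string.
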(event OnBeginInteracted(MamontBoxInteractable)
  (params (InInstigator :type Actor%20Object%20Reference))
  (CallFunction|StartDialogue InInstigator)
  (Development|PrintString "Dialogue"))

(event Custom|OnMayTalk
  (Collision|SetCollisionEnabled (Variables|Default|GetMamontBoxInteractable) "QueryOnly"))

(event EventBeginPlay
  (bind _returnvalue (Class|CombatManagerInterface|GetCombatManagerComponent(Message) (Game|GetGameState)))
  (Utilities|IsValid _returnvalue
    (:Is%20Valid
      (EventDispatchers|BindEventtoOnDeadAllEnemyCharacters _returnvalue (EventDispatchers|CreateEvent :!event Custom|OnMayTalk)))))

(fn ConstructionScript)

(fn StartDialogue
  (params (InInstigator :type Actor%20Object%20Reference))
  (Class|DialogueSpeakerComponent|StartOwnedDialogue (Variables|Default|GetBPC_SpeakerComponent) (Utilities|Array|MakeArray (Actor|GetComponentbyClass InInstigator "/Script/DialogueTreeRuntime.DialogueSpeakerComponent"))))