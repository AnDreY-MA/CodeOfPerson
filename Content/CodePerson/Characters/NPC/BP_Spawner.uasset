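; BP_Spawner is an NPC spawner that places copies of SpawnCharacter at random navigable spots around itself.
; Spawn runs one second after BeginPlay when SpawnBegin is set, and is also a standalone event.
; It loops based on Count, async-loading the soft class on each pass.
; Each completed load spawns an actor at a random reachable point within Radius, using the spawner's rotation.
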(event EventBeginPlay
  (if (Variables|Default|GetbSpawnBegin)
    (Utilities|FlowControl|Delay 1.0)
    (Class|Spawner|Spawn)))

(event EventSpawn
  (bind _returnvalue (Transformation|GetActorTransform))
  (for _index (range 0 (Variables|Default|GetCount))
    (bind _class (Utilities|AsyncLoadClassAsset (Variables|Default|GetSpawnCharacter))
      (:Completed
        (bind _asactor (Utilities|Casting|CastToActorClass _class))
        (Game|SpawnActorfromClass _asactor (Math|Transform|MakeTransform (.RandomLocation (AI|Navigation|GetRandomReachablePointinRadius (.location _returnvalue) (Variables|Default|GetRadius) 0 0)) (.rotation _returnvalue) "1.000000,1.000000,1.000000") "Undefined" "MultiplyWithRoot" 0 0)))))

(fn ConstructionScript)