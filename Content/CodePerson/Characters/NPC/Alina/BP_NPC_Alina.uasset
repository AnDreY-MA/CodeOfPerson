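; Alina NPC Blueprint that plays scripted actions: a down animation and walking to a bunny to pick it up.
; The down montage fires a completion dispatcher when it completes or blends out.
; The pickup uses AI MoveTo, sets a motion-warp target at the bunny, plays a montage, then enables query collision on MamontBoxInteractable.
; A separate GrabBunny event disables the bunny's mesh collision and attaches it to the hand socket.
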(event Custom|PlayDownAnimation
  (Animation|Montage|PlayMontage (Variables|Character|GetMesh) "/Game/CodePerson/Characters/NPC/Alina/AM_Alina_Down.AM_Alina_Down"
    (:OnCompleted
      _)
    (:OnBlendOut
      _))
  (Default|CallOnDownAnimCompleted))

(event Custom|MoveToBunnyAndPickUp
  (params (GoalActor :type Actor%20Object%20Reference))
  (Development|PrintString (Utilities|GetDisplayName GoalActor))
  (bind _output_get (Variables|Default|SetBunny GoalActor))
  (AI|AIMoveTo (AI|GetAIController self) "0, 0, 0" _output_get 1.0 "Default" "Default" true true
    (:OnRequestFailed
      (Development|PrintString "MoveBunnyFail"))
    (:OnMoveFinished
      (Class|MotionWarpingComponent|AddorUpdateWarpTargetfromLocationandRotation (Variables|Default|GetMotionWarping) "BunnyTarget" (Transformation|GetActorLocation _output_get) "0, 0, 0")
      (Animation|Montage|PlayMontage (Variables|Character|GetMesh) "/Game/CodePerson/Characters/NPC/Alina/AM_Alina_PickupBunny.AM_Alina_PickupBunny"
        (:OnCompleted
          _)
        (:OnBlendOut
          _))
      (Collision|SetCollisionEnabled (Variables|Default|GetMamontBoxInteractable) "QueryOnly"))))

(event EventGrabBunny
  (bind _bunny (Variables|Default|GetBunny)
    (:then
      (Collision|SetCollisionEnabled (Actor|GetComponentbyClass _bunny "/Script/Engine.StaticMeshComponent") "NoCollision")
      (Transformation|AttachComponentToComponent _bunny (Variables|Character|GetMesh) "BunnyHand_Socket" "SnapToTarget" "SnapToTarget" "KeepRelative" true))
    (:else)))

(event EventBeginPlay
  (|CallParentFunction))

(fn ConstructionScript
  (|CallParentFunction))