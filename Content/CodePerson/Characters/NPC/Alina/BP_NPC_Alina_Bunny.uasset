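; Alina's bunny NPC Blueprint, present in the world only when the game data holds the Narrative.AlinaBunny key.
; Shortly after BeginPlay, the HasBunny check queries the GameInstance's game data message and switches the capsule's activation, collision and propagated visibility on or off.
; A separate SwitchVisibl helper, not called here, sets capsule collision and disables collision on MamontBoxInteractable.
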(event EventBeginPlay
  (bind _capsulecomponent (Variables|Default|GetCapsuleComponent))
  (|CallParentFunction)
  (Utilities|FlowControl|Delay 0.2)
  (Utilities|HasBunny
    (:true
      (Components|Activation|SetActive _capsulecomponent true false)
      (Collision|SetCollisionEnabled _capsulecomponent "QueryAndPhysics")
      (Rendering|SetVisibility _capsulecomponent true true))
    (:false
      (Components|Activation|SetActive _capsulecomponent false false)
      (Collision|SetCollisionEnabled _capsulecomponent "NoCollision")
      (Rendering|SetVisibility _capsulecomponent false true))))

(fn ConstructionScript
  (|CallParentFunction))

(fn GetCombatWarpingComponent
  (return 0))