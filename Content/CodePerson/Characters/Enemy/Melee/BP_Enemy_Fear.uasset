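; BP_Enemy_Fear is a melee enemy character Blueprint that extends its parent's setup with weapon-based combat tracing.
; On BeginPlay it runs the parent logic, then points its CombatTrace component at the static mesh inside its child actor.
; Two getters expose its CombatSystem and CombatTrace components, and the construction script only calls the parent.
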(event EventBeginPlay
  (|CallParentFunction)
  (Class|CombatTraceComponent|ChangeTracingComponent (Variables|Default|GetCombatTrace) (Actor|GetComponentbyClass (Variables|/Script/Engine.ChildActorComponent|GetChildActor (Variables|Default|GetChildActor)) "/Script/Engine.StaticMeshComponent")))

(fn ConstructionScript
  (|CallParentFunction))

(fn GetCombatSystemComponent
  (return (Variables|Default|GetCombatSystem)))

(fn GetCombatTraceComponent
  (return (Variables|Default|GetCombatTrace)))