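; BP_Enemy is an enemy Blueprint that works out which side a hit or incoming position is on.
; GetHitDirection compares that position's distance to four arrow components (left, back, front, right) and returns the closest arrow.
; Its second enum output is fixed to one value, as the Select that would vary it is unconnected.
; GetDirection wraps it, exposing only the arrow.
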(fn ConstructionScript)

(fn GetHitDirection
  (params (InDirection :type Vector))
  (Utilities|FlowControl|DoOnce false :!label _label
    (:Completed
      (for (_array_element _array_index) (Utilities|Array|MakeArray (Math|Vector|Distance(Vector) InDirection (Transformation|GetWorldLocation (Variables|Default|GetLeftArrow))) (Math|Vector|Distance(Vector) InDirection (Transformation|GetWorldLocation (Variables|Default|GetBackArrow))) (Math|Vector|Distance(Vector) InDirection (Transformation|GetWorldLocation (Variables|Default|GetFrontArrow))) (Math|Vector|Distance(Vector) InDirection (Transformation|GetWorldLocation (Variables|Default|GetRightArrow))))
        (Math|Float|CompareFloat _array_element (LocalVariables|GetClossetArrowDistane%20%28local%29)
          (:<
            (LocalVariables|SetClossetArrowDistane%20%28local%29 _array_element)
            (LocalVariables|SetIndexClosset%28local%29 _array_index))))
      (Utilities|FlowControl|Sequence
        (:then_0
          (goto _label Reset))
        (:then_1
          (return (Utilities|Select :Index (LocalVariables|GetIndexClosset%28local%29) :Option%200 (Variables|Default|GetLeftArrow) :Option%201 (Variables|Default|GetBackArrow) :Option%202 (Variables|Default|GetFrontArrow) :Option%203 (Variables|Default|GetRightArrow)) "NewEnumerator0"))))))

(fn GetDirection
  (params (InDirection :type Vector%20%28by%20ref%29 :default "0, 0, 0"))
  (return (.OutDirection (CallFunction|GetHitDirection InDirection))))