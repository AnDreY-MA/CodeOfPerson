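; Enemy boss Blueprint for the Bunny boss, extending a parent class with combat UI, trace and warping components.
; On BeginPlay it points CombatTrace at its Mesh, then after a short delay prints a float attribute from its CombatSystemComponent ability system as on-screen debug text.
; Getter functions expose the CombatUI, CombatTrace and CombatWarping components to callers.
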(event EventBeginPlay
  (|CallParentFunction)
  (Class|CombatTraceComponent|ChangeTracingComponent (Variables|Default|GetCombatTrace) (Variables|Character|GetMesh))
  (Utilities|FlowControl|Delay 1.0)
  (Development|PrintString (Utilities|String|ToString(Float) (.ReturnValue (Ability|Attribute|GetFloatAttributefromAbilitySystemComponent (Variables|Default|GetCombatSystemComponent) "(AttributeName=\"Health\",Attribute=/Script/CombatAbilitiesSystem.CombatAttributeSet:Health,AttributeOwner=\"/Script/CoreUObject.Class'/Script/CombatAbilitiesSystem.CombatAttributeSet'\")"))) true true "(R=1.000000,G=0.611447,B=0.000000,A=1.000000)" 5.0))

(fn ConstructionScript
  (|CallParentFunction))

(fn GetCombatUIComponent
  (return (Variables|Default|GetCombatUI)))

(fn GetCombatTraceComponent
  (return (Variables|Default|GetCombatTrace)))

(fn GetCombatWarpingComponent
  (return (Variables|Default|GetCombatWarping)))