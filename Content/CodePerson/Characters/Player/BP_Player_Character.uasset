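; Player character Blueprint with Enhanced Input movement, interaction and sword combat components.
; The interact input, gated by BPCInteraction, messages the first overlapping actor and also triggers MamontInteraction.
; BeginPlay points CombatTrace at the Sword child actor's static mesh and shows the cursor, printing an error if the mesh is invalid.
; Getters expose CombatTrace and CombatWarping; a helper, uncalled in these graphs, turns the character toward the cursor hit point.
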(event Input|EnhancedActionEvents|EnhancedInputActionIA_Move
  (params (ActionValue :type Vector%202D%20Structure) (ElapsedSeconds :type Float%20%28double-precision%29) (TriggeredSeconds :type Float%20%28double-precision%29) (InputAction :type Input%20Action%20Object%20Reference :default "/Game/CodePerson/Controllers/Player/Input/Actions/IA_Move.IA_Move"))
  (Class|CodePersonCharacter|Move (Class|EnhancedInputLibrary|MakeInputActionValueOfType (.x ActionValue) (.y ActionValue) 0.0 "Axis2D")))

(event Input|EnhancedActionEvents|EnhancedInputActionIA_Interaction
  (params (ActionValue :type Boolean) (ElapsedSeconds :type Float%20%28double-precision%29) (TriggeredSeconds :type Float%20%28double-precision%29) (InputAction :type Input%20Action%20Object%20Reference :default "/Game/CodePerson/Controllers/Player/Input/Actions/IA_Interaction.IA_Interaction"))
  (if (Default|GetCanInteract (Variables|Default|GetBPC_Interaction))
    (CallFunction|TryInteract)
    (Class|MamontInteractionComponent|InteractonOverlap (Variables|Default|GetMamontInteraction))))

(event EventBeginPlay
  (bind _sword (Variables|Default|GetSword))
  (bind _childactor (Variables|/Script/Engine.ChildActorComponent|GetChildActor _sword))
  (bind _returnvalue (Actor|GetComponentbyClass _childactor "/Script/Engine.StaticMeshComponent"))
  (Utilities|IsValid _returnvalue
    (:Is%20Valid
      (Class|CombatTraceComponent|ChangeTracingComponent (Variables|Default|GetCombatTrace) _returnvalue)
      (Variables|/Script/Engine.PlayerController|SetbShowMouseCursor (Game|GetPlayerController 0) true))
    (:Is%20Not%20Valid
      (Development|PrintString (Utilities|String|Append "StaticMesh —" "NoValid") true true "(R=1.000000,G=0.063102,B=0.000000,A=1.000000)"))))

(fn ConstructionScript)

(fn RotatetoMousPosition
  (params (DeltaTime :type Float%20%28single-precision%29))
  (bind _returnvalue (Game|GetPlayerController 0))
  (bind _returnvalue_2 (Transformation|GetActorLocation))
  (bind _hitresult (Game|Player|GetHitResultUnderCursorbyChannel _returnvalue "TraceTypeQuery1" true))
  (bind (_x _y) (Math|Vector|BreakVector (.location _hitresult)))
  (Variables|Default|SetLookLocation (Math|Rotator|FindLookatRotation (Math|Vector|MakeVector (.x _returnvalue_2) (.y _returnvalue_2) 0.0) (Math|Vector|MakeVector _x _y 0.0)))
  (Transformation|SetActorRotation (Class|KismetMathLibrary|RInterptoConstant (Transformation|GetActorRotation) (Variables|Default|GetLookLocation) DeltaTime 1.8e+02)))

(fn TryInteract
  (bind _overlappingactors (Collision|GetOverlappingActors "/Script/Engine.Character" :!class /Script/Engine.Actor))
  (bind _overlappingactors_2 (Collision|GetOverlappingActors "/Script/Engine.Actor" :!class /Script/Engine.Actor))
  (Utilities|FlowControl|Sequence
    (:then_0
      (if (not (Utilities|Array|IsEmpty _overlappingactors))
        (LocalVariables|SetActorsInteract%20%28local%29 _overlappingactors)))
    (:then_1
      (if (not (Utilities|Array|IsEmpty _overlappingactors_2))
        (LocalVariables|SetActorsInteract%20%28local%29 _overlappingactors_2)))
    (:then_2
      (if (and (Utilities|Array|IsNotEmpty (LocalVariables|GetActorsInteract%20%28local%29)) (Utilities|Array|IsValidIndex (LocalVariables|GetActorsInteract%20%28local%29)))
        (Class|InteractableInterface|Interact(Message) (Utilities|Array|Get(acopy) (LocalVariables|GetActorsInteract%20%28local%29)) self)))))

(fn GetCombatWarpingComponent
  (return (Variables|Default|GetCombatWarping)))

(fn GetCombatTraceComponent
  (return (Variables|Default|GetCombatTrace)))