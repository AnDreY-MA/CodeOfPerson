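; Sword weapon Blueprint for player characters that adds a colored trail effect to the blade.
; On BeginPlay, after the parent logic, it attaches the FXS_SwordTrail system to the static mesh, centered between the TrailStart and TrailEnd sockets and oriented along them.
; The socket distance drives the trail width, and the TrailColor variable sets its color.
; An alternative SetVariableLinearColor call is left unconnected.
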(event EventBeginPlay
  (bind _staticmesh (Variables|Default|GetStaticMesh))
  (bind _returnvalue (Transformation|GetSocketLocation _staticmesh "TrailStart"))
  (bind _returnvalue_2 (Transformation|GetSocketLocation _staticmesh "TrailEnd"))
  (bind _returnvalue_3 (- _returnvalue_2 _returnvalue))
  (|CallParentFunction)
  (bind _returnvalue_4 (Niagara|SpawnSystemAttached "/Game/CodePerson/Characters/Player/Weapons/Effects/FXS_SwordTrail.FXS_SwordTrail" (Variables|Default|GetStaticMesh) "None" (/ (+ _returnvalue_2 _returnvalue) 2.0) (Math|Rotator|MakeRotfromZ _returnvalue_3) "KeepWorldPosition" true))
  (Effects|Components|ParticleSystem|SetFloatParameter _returnvalue_4 "TrailWidth" (Math|Vector|VectorLength _returnvalue_3))
  (Effects|Components|ParticleSystem|SetColorParameter _returnvalue_4 "TrailColor" (Variables|Default|GetTrailColor)))

(fn ConstructionScript)