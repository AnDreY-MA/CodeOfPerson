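; Gameplay ability that handles a character's death and destroys the avatar when it ends.
; Activation from an event makes the capsule ignore a custom trace channel, stops AI brain logic, and plays a random death montage from the combat component interface, selected by gameplay tag.
; Any montage outcome ends the ability.
; A separate DropLoot event, not called here, async-loads the loot class and spawns it at the owner's location.
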(event Custom|DropLoot
  (Utilities|AsyncLoadClassAsset (Variables|Default|GetLootActorClass)
    (:Completed
      (Game|SpawnActorfromClass (Utilities|ResolveSoftReference (Variables|Default|GetLootActorClass)) (Math|Conversions|ToTransform(Vector) (Transformation|GetActorLocation (Ability|GetOwningActorfromActorInfo))) "Undefined" "MultiplyWithRoot" 0 0))))

(event Ability|EventOnEndAbility
  (params (bWasCancelled :type Boolean))
  (Actor|DestroyActor (Ability|GetAvatarActorfromActorInfo))
  (|CallParentFunction bWasCancelled))

(event Ability|EventActivateAbilityFromEvent
  (params (EventData :type Gameplay%20Event%20Data%20Structure%20%28by%20ref%29))
  (bind _returnvalue (Ability|GetAvatarActorfromActorInfo))
  (bind _returnvalue_2 (AI|GetAIController _returnvalue))
  (bind _returnvalue_3 (Actor|GetComponentbyClass _returnvalue_2 "/Script/AIModule.BrainComponent"))
  (Collision|SetCollisionResponsetoChannel (Actor|GetComponentbyClass _returnvalue "/Script/Engine.CapsuleComponent") "ECC_GameTraceChannel1" "ECR_Ignore")
  (Utilities|IsValid _returnvalue_3
    (:Is%20Valid
      (AI|Logic|StopLogic _returnvalue_3 ""))
    (:Is%20Not%20Valid
      _))
  (bind _returnvalue_4 (Class|CombatComponentInterface|GetMontageAction(Message) (Utilities|Array|Get(acopy) (Class|Actor|GetComponentsbyInterface (Ability|GetAvatarActorfromActorInfo) "/Script/CombatAbilitiesSystem.CombatComponentInterface")) (GameplayTags|MakeLiteralGameplayTag "(TagName=\"CombatAbilities.Death\")")))
  (|PlayMontageandWaitforEvent :MontageToPlay (.Montage (Utilities|Struct|BreakCombatAnimationInfo (.OutItem (Utilities|Array|Random _returnvalue_4)))) :Rate (.Speed (Utilities|Struct|BreakCombatAnimationInfo (.OutItem (Utilities|Array|Random _returnvalue_4))))
    (:OnCompleted
      _)
    (:OnBlendOut
      _)
    (:OnInterrupted
      _)
    (:OnCancelled
      _))
  (Ability|EndAbility))