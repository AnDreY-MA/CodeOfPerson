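; GA_HitReact is an event-triggered Gameplay Ability that gives the hit character a short knockback and material flash.
; It applies a brief root motion move-to-actor force targeting its own owner, offset along the instigator's forward vector scaled by a strength variable.
; Once the force starts, it stops movement and raises an emissive hit parameter on the mesh materials.
; It ends after a short delay, resetting that parameter.
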(event Ability|EventOnEndAbility
  (params (bWasCancelled :type Boolean))
  (Rendering|Material|SetScalarParameterValueonMaterials (Class|GameplayAbility|GetOwningComponentfromActorInfo) "EmissiveHit" 0.0))

(event Ability|EventActivateAbilityFromEvent
  (params (EventData :type Gameplay%20Event%20Data%20Structure%20%28by%20ref%29))
  (bind _returnvalue (Ability|GetActorInfo))
  (bind (_owneractor _avataractor _playercontroller _abilitysystemcomponent _skeletalmeshcomponent _animinstance _movementcomponent) (Utilities|Struct|BreakGameplayAbilityActorInfo _returnvalue))
  (Ability|Tasks|ApplyRootMotionMoveToActorForce "None" _owneractor (* (Transformation|GetActorForwardVector (Utilities|Struct|BreakGameplayEventData EventData)) (Variables|Default|GetStrenght)) "AlignFromTargetToSource" 0.1 0 0 false "MOVE_None" false 0 0 "MaintainLastRootMotionVelocity"
    (:then
      (Components|Movement|StopMovementImmediately _movementcomponent)
      (Rendering|Material|SetScalarParameterValueonMaterials (Class|GameplayAbility|GetOwningComponentfromActorInfo) "EmissiveHit" 1.0)
      (Utilities|FlowControl|Delay 0.2)
      (Ability|EndAbility))))