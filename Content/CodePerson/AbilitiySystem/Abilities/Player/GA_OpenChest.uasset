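; Player gameplay ability that plays a chest-opening montage and opens a nearby chest.
; On activation it starts async-loading the montage while a sphere trace around the avatar finds a chest and sets it as the motion-warp target.
; After loading and a short delay it plays the montage, calls Open on the chest when the BrokeChest event arrives, and ends when the montage finishes or is interrupted.
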(event Ability|EventActivateAbility
  (bind _returnvalue (Ability|GetAvatarActorfromActorInfo))
  (bind _returnvalue_2 (Transformation|GetActorLocation _returnvalue))
  (bind _object (Utilities|AsyncLoadAsset (Variables|Default|GetMontage))
    (:then
      (bind (_outhit _returnvalue_3) (Collision|SphereTraceByChannel _returnvalue_2 _returnvalue_2 1e+02 "TraceTypeQuery1" false 0 "ForDuration"))
      (if _returnvalue_3
        (bind _aschests (Utilities|Casting|CastToChests (.HitActor (Collision|BreakHitResult _outhit))))
        (bind _output_get (Variables|Default|SetChests _aschests))
        (bind _returnvalue_4 (Class|CombatWarpComponentInterface|GetCombatWarpingComponent(Message) (Ability|GetAvatarActorfromActorInfo)))
        (Class|MotionWarpingComponent|AddorUpdateWarpTargetfromLocationandRotation _returnvalue_4 (Variables|Default|GetWarp%20Target%20Name) (Transformation|GetActorLocation _output_get) "0, 0, 0")))
    (:Completed
      (Utilities|FlowControl|Delay 0.1)
      (bind _asanim_montage (Utilities|Casting|CastToAnimMontage _object))
      (|PlayMontageandWaitforEvent "None" _asanim_montage "(GameplayTags=((TagName=\"Events.BrokeChest\")))" 1.0 "None" true 1.0
        (:OnCompleted
          (Ability|EndAbility :!label _label))
        (:OnBlendOut
          (goto _label))
        (:OnInterrupted
          (goto _label))
        (:OnCancelled
          (goto _label))
        (:EventReceived
          (Class|Chests|Open (Variables|Default|GetChests)))))))