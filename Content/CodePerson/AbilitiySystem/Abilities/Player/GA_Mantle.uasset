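; Player mantle ability that moves the avatar onto obstacles using traced positions and motion warping.
; A forward line trace and follow-up sphere traces compute two mantle points and decide whether mantling is possible.
; Mantle disables collision, switches to Flying, sets both points as warp targets, then plays an async-loaded montage.
; After a montage-length delay, it restores collision and switches movement to Falling.
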(event Ability|EventActivateAbility
  (Variables|Default|SetAvatar (Ability|GetAvatarActorfromActorInfo))
  (bind (_outlocation1 _outlocation2) (CallFunction|Trace))
  (if (Variables|Default|GetCanMantle)
    (Utilities|Mantle _outlocation1 _outlocation2)
    (Ability|EndAbility)
    (else
      (Ability|EndAbility))))

(fn Trace
  (bind _avatar (Variables|Default|GetAvatar))
  (bind _returnvalue (Transformation|GetActorLocation _avatar))
  (Variables|Default|SetCanMantle false)
  (bind (_outhit _returnvalue_2) (Collision|LineTraceByChannel _returnvalue (+ _returnvalue (* (Transformation|GetActorForwardVector (Variables|Default|GetAvatar)) (Variables|Default|GetInitTraceLength))) "TraceTypeQuery4" false 0 "ForDuration"))
  (if _returnvalue_2
    (bind (_outhit_2 _returnvalue_3) (Collision|SphereTraceByChannel (.Location (Collision|BreakHitResult _outhit)) (+ (.Location (Collision|BreakHitResult _outhit)) (Math|Vector|MakeVector 0.0 0.0 (* (Variables|Default|GetSecondaryTraceZ) (Variables|Default|GetFallingHeightMultiplier)))) 1e+01 "TraceTypeQuery4" false 0 "ForDuration"))
    (if _returnvalue_3
      (LocalVariables|SetMantlePosition1%28local%29 (+ (.ImpactPoint (Collision|BreakHitResult _outhit_2)) (* (Transformation|GetActorForwardVector (Variables|Default|GetAvatar)) (LocalVariables|GetMultiplierImapcPos1))))
      (bind _output_get (LocalVariables|SetMantlePosition2%28local%29 (+ (* (Transformation|GetActorForwardVector (Variables|Default|GetAvatar)) 1.2e+02) (.ImpactPoint (Collision|BreakHitResult _outhit_2)))))
      (Variables|Default|SetCanMantle true)
      (bind _returnvalue_4 (Collision|SphereTraceByChannel (+ _output_get "0.000000,0.000000,20.000000") (+ _output_get "0.000000,0.000000,20.000000") 1e+01 "TraceTypeQuery4" false 0 "ForDuration"))
      (if _returnvalue_4
        (Variables|Default|SetCanMantle false)
        (else
          (LocalVariables|SetMantlePosition2%28local%29 (+ (.ImpactPoint (Collision|BreakHitResult _outhit_2)) (* (Transformation|GetActorForwardVector (Variables|Default|GetAvatar)) 5e+01)))))
      (if (or (Utilities|Operators|EqualEqual :A (LocalVariables|GetMantlePosition1%28local%29)) (Utilities|Operators|EqualEqual :A (LocalVariables|GetMantlePosition2%28local%29)))
        (Variables|Default|SetCanMantle true :!label _label)
        (return (LocalVariables|GetMantlePosition1%28local%29) (LocalVariables|GetMantlePosition2%28local%29))
        (else
          (bind _returnvalue_5 (Collision|SphereTraceByChannel (Math|Vector|MakeVector (.x (LocalVariables|GetMantlePosition1%28local%29)) (.y (LocalVariables|GetMantlePosition1%28local%29)) 0.0) (+ (LocalVariables|GetMantlePosition2%28local%29) "0.000000,0.000000,100.000000") 2e+01 "TraceTypeQuery4" false 0 "ForDuration"))
          (if _returnvalue_5
            (goto _label)))))
    (else
      (Variables|Default|SetCanMantle false))))