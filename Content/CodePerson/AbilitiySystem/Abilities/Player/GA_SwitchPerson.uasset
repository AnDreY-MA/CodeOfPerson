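; Gameplay ability that toggles the player between the Aya and Rangard personas, then ends immediately.
; It branches on the controller's current persona and switches to the other by gameplay tag.
; Each switch retargets the avatar's combat trace component to the skeletal mesh for Rangard or the tagged Sword child actor's static mesh for Aya.
; It also swaps the footstep component's triggered layer types to match the new persona.
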(event Ability|EventActivateAbility
  (Variables|Default|SetAvatarOwner (Ability|GetAvatarActorfromActorInfo))
  (bind _outpersoncomponent (Utilities|PersonSelect (.playercontroller (Ability|GetActorInfo)))
    (:Persons.Aya
      ;[1 1 1] Rangard
      (Class|PersonComponent|SwitchPerson _outpersoncomponent (GameplayTags|MakeLiteralGameplayTag "(TagName=\"Persons.Rangard\")"))
      (Utilities|ChangeTracingComponent (Actor|GetComponentbyClass (Variables|Default|GetAvatarOwner) "/Script/Engine.SkeletalMeshComponent"))
      (Utilities|ChangeFootStepsType (Variables|Default|GetRangard%20Layers%20Types)))
    (:Persons.Rangard
      ;[1 1 1] Aya
      (Class|PersonComponent|SwitchPerson _outpersoncomponent (GameplayTags|MakeLiteralGameplayTag "(TagName=\"Persons.Aya\")"))
      (Utilities|ChangeTracingComponent (Actor|GetComponentbyClass (Variables|/Script/Engine.ChildActorComponent|GetChildActor (Class|Actor|FindComponentbyTag (Variables|Default|GetAvatarOwner) "/Script/Engine.ChildActorComponent" "Sword")) "/Script/Engine.StaticMeshComponent"))
      (Utilities|ChangeFootStepsType (Variables|Default|GetAya%20Layers%20Types))))
  (Ability|EndAbility))