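; Death gameplay ability for the bunny boss, which leaves a crying bunny prop in place of the defeated boss.
; Event-triggered activation is passed straight to the parent ability.
; When the ability ends, it calls the boss's OnDefeat and spawns a movable static mesh actor tagged "Bunny" at the skeletal mesh's location and rotation.
; The boss avatar then gets a near-zero lifespan, so it is destroyed almost immediately.
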(event EventActivateAbilityfromEvent
  (params (EventData :type Gameplay%20Event%20Data%20Structure%20%28by%20ref%29))
  (|CallParentFunction EventData))

(event Ability|EventOnEndAbility
  (params (bWasCancelled :type Boolean))
  (bind _returnvalue (Ability|GetActorInfo))
  (bind _asbp_enemy_boss_bunny (Utilities|Casting|CastToBP_Enemy_Boss_Bunny (Ability|GetAvatarActorfromActorInfo)))
  (Default|CallOnDefeat _asbp_enemy_boss_bunny)
  (bind _returnvalue_2 (Game|SpawnActorfromClass "/Script/Engine.StaticMeshActor" (Math|Transform|MakeTransform (Transformation|GetWorldLocation (.skeletalmeshcomponent _returnvalue)) (Transformation|GetWorldRotation (.skeletalmeshcomponent _returnvalue)) "1.000000,1.000000,1.000000") "Undefined" "MultiplyWithRoot" 0 0))
  (Variables|/Script/Engine.Actor|SetTags _returnvalue_2 (Utilities|Array|MakeArray "Bunny"))
  (Transformation|SetMobility (Variables|/Script/Engine.StaticMeshActor|GetStaticMeshComponent _returnvalue_2) "Movable")
  (Components|StaticMesh|SetStaticMesh (Variables|/Script/Engine.StaticMeshActor|GetStaticMeshComponent _returnvalue_2) "/Game/CodePerson/Characters/Enemy/Bosses/Bunny/Mesh/SM_Bunny_CryIdle.SM_Bunny_CryIdle")
  (Actor|SetLifeSpan (Ability|GetAvatarActorfromActorInfo) 0.0001))