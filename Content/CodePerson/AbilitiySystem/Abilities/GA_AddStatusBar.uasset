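; GA_AddStatusBar is a Gameplay Ability that puts a combat status widget on screen.
; On activation it async-loads the StatWidget class, creates the widget and adds it to the viewport.
; It initializes the widget with the controller of the avatar actor's Instigator, then ends.
; An invalid StatWidget ends the ability immediately, while a failed class cast stops without ending it.
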(event Ability|EventActivateAbility
  (bind _statwidget (Variables|Default|GetStatWidget)
    (:then
      (bind _class (Utilities|AsyncLoadClassAsset _statwidget)
        (:Completed
          (bind _ascombat_status_widget (Utilities|Casting|CastToCombatStatusWidgetClass _class))
          (bind _returnvalue (UserInterface|CreateWidget _ascombat_status_widget))
          (UserInterface|Viewport|AddtoViewport _returnvalue 0)
          (Class|CombatStatusWidget|InitWidgetfromActor _returnvalue (Pawn|GetController (Variables|/Script/Engine.Actor|GetInstigator (Ability|GetAvatarActorfromActorInfo))))
          (Ability|EndAbility))))
    (:else
      (Ability|EndAbility))))