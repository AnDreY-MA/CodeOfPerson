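; BP_Projectile_Bullet is a projectile that adds effects and a physical impulse to the spawn and hit behavior of its parent class.
; On BeginPlay it spawns an optional particle system at its own location and rotation.
; On hit it calls the parent handler, fires its RadialForce impulse, spawns a hit emitter, plays the Laser_Pull sound and destroys itself.
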(event EventBeginPlay
  (|CallParentFunction)
  (Utilities|IsValid (Variables|NiagaraEffects|GetSpawningEffect)
    (:Is%20Valid
      (Niagara|SpawnSystematLocation (Variables|NiagaraEffects|GetSpawningEffect) (Transformation|GetActorLocation) (Transformation|GetActorRotation)))))

(event EventOnProjectileHit
  (params (HitComponent :type Primitive%20Component%20Object%20Reference) (OtherActor :type Actor%20Object%20Reference) (OtherComp :type Primitive%20Component%20Object%20Reference) (NormalImpulse :type Vector :default "0, 0, 0") (Hit :type Hit%20Result%20Structure%20%28by%20ref%29))
  (bind _returnvalue (Transformation|GetActorLocation))
  (|CallParentFunction HitComponent OtherActor OtherComp NormalImpulse Hit)
  (Class|RadialForceComponent|FireImpulse (Variables|Default|GetRadialForce))
  (Effects|SpawnEmitteratLocation (Variables|NiagaraEffects|GetHitEffect) _returnvalue)
  (Audio|PlaySoundatLocation "/Engine/VREditor/Sounds/UI/Laser_Pull.Laser_Pull" _returnvalue "0, 0, 0" 1.0 1.0 0.0 0 0 0 0)
  (Actor|DestroyActor))

(fn ConstructionScript)